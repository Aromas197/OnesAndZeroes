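; Speed trigger actor that boosts the player's walk speed while an overlap is active.
; Overlap begin sets player 0's MaxWalkSpeed to GetMaxSpeed plus a fixed amount, and overlap end sets it to GetMaxSpeed minus the same amount.
; The overlapping actor is not checked, so any overlap alters the player's speed.
; No original speed is stored, and GetMaxSpeed depends on the current movement mode.
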(event `self.ReceiveActorBeginOverlap`
  (params (OtherActor :type "Actor Object Reference"))
  (bind _charactermovement (`Character.CharacterMovement` (`GameplayStatics.GetPlayerCharacter` 0)))
  (set `CharacterMovementComponent.MaxWalkSpeed` (+ (`MovementComponent.GetMaxSpeed` _charactermovement) 600.0) _charactermovement))

(event `self.ReceiveActorEndOverlap`
  (params (OtherActor :type "Actor Object Reference"))
  (bind _charactermovement (`Character.CharacterMovement` (`GameplayStatics.GetPlayerCharacter` 0)))
  (set `CharacterMovementComponent.MaxWalkSpeed` (- (`MovementComponent.GetMaxSpeed` _charactermovement) 600.0) _charactermovement))

(fn `UserConstructionScript`)