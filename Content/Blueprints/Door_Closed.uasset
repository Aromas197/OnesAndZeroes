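; A 2D flipbook door that opens as an actor overlaps it and moves the player to a fixed location when F is pressed.
; Begin and end overlap set an overlap flag and play the opening or closing flipbook.
; After a delay of the flipbook's length, both paths pick the open or closed flipbook from that flag.
; The F action requires both the flag and a looping flipbook, which the overlap events toggle.
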(event `Key|F`
  (params (Key :type "Key Structure"))
  (:`Pressed`
    (if (and (`self.playerIsOverlapping`) (`PaperFlipbookComponent.IsLooping` (`self.RenderComponent`)))
      (`self.K2_SetActorLocation` (`GameplayStatics.GetPlayerPawn` 0) (-62.0 0.0 865.0) false false))))

(event `self.ReceiveBeginPlay`
  (`self.EnableInput` (`GameplayStatics.GetPlayerController` 0)))

(event `self.ReceiveActorBeginOverlap`
  (params (OtherActor :type "Actor Object Reference"))
  (bind _rendercomponent (`self.RenderComponent`))
  (`PaperFlipbookComponent.SetLooping` _rendercomponent true)
  (`PaperFlipbookComponent.SetFlipbook` _rendercomponent "/Game/Env/Door/Door_Opening.Door_Opening")
  (set `self.playerIsOverlapping` true)
  (`PaperFlipbookComponent.Play` _rendercomponent)
  (`KismetSystemLibrary.Delay` (`PaperFlipbookComponent.GetFlipbookLength` _rendercomponent))
  (if (`self.playerIsOverlapping`) :!label _label
    (`PaperFlipbookComponent.SetFlipbook` _rendercomponent "/Game/Env/Door/Door_Open.Door_Open")
    (else
      (`PaperFlipbookComponent.SetFlipbook` _rendercomponent "/Game/Env/Door/Door_Closed.Door_Closed"))))

(event `self.ReceiveActorEndOverlap`
  (params (OtherActor :type "Actor Object Reference"))
  (bind _rendercomponent (`self.RenderComponent`))
  (`PaperFlipbookComponent.SetLooping` _rendercomponent false)
  (`PaperFlipbookComponent.SetFlipbook` _rendercomponent "/Game/Env/Door/Door_Closing.Door_Closing")
  (set `self.playerIsOverlapping` false)
  (`PaperFlipbookComponent.Play` _rendercomponent)
  (`KismetSystemLibrary.Delay` (`PaperFlipbookComponent.GetFlipbookLength` _rendercomponent))
  (goto _label))

(fn `UserConstructionScript`)